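; BP_Grid procedurally grows a random, connected layout of BP_Cell tiles on a flat grid at BeginPlay.
; After a short delay it spawns a seed cell, then repeatedly spawns cells at random open positions.
; After each spawn it records occupied locations, adds every cell's four neighbors at Largeur spacing, and filters out occupied ones with a small tolerance.
; Unconnected leftover direction-picking logic never runs.
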(event `self.ReceiveBeginPlay`
  (`KismetSystemLibrary.Delay` 0.5)
  (bind _returnvalue (`|SpawnActorFromClass` "/Game/Procedural/Blueprint/BP_Cell.BP_Cell_C" (`KismetMathLibrary.MakeTransform` (0.0 0.0 0.0)) "Undefined" "MultiplyWithRoot" null null))
  (`KismetArrayLibrary.Array_AddUnique` (`self.CellArray`) _returnvalue)
  (`self.SetForbidenPosition`)
  (for _ (range (+ (`self.TileToSapwn`) 1))
    (`self.SpawnNewTile`)))

(event `self.ReceiveTick`
  (params (DeltaSeconds :type "Float (single-precision)")))

(fn `AddAvailablePsoition`
  (for _array_element (`self.CellArray`)
    (bind (_returnvalue_x _returnvalue_y) (`KismetMathLibrary.BreakVector` (`self.K2_GetActorLocation` _array_element)))
    (bind _largeur (`/Game/Procedural/Blueprint/BP_Cell.Largeur` _array_element))
    (`KismetArrayLibrary.Array_AddUnique` (`self.AvailablePosition`) (`KismetMathLibrary.MakeVector` (+ _returnvalue_x _largeur) _returnvalue_y))
    (`KismetArrayLibrary.Array_AddUnique` (`self.AvailablePosition`) (`KismetMathLibrary.MakeVector` (- _returnvalue_x _largeur) _returnvalue_y))
    (`KismetArrayLibrary.Array_AddUnique` (`self.AvailablePosition`) (`KismetMathLibrary.MakeVector` _returnvalue_x (+ _returnvalue_y _largeur)))
    (`KismetArrayLibrary.Array_AddUnique` (`self.AvailablePosition`) (`KismetMathLibrary.MakeVector` _returnvalue_x (- _returnvalue_y _largeur))))
  (`KismetSystemLibrary.PrintString` (`KismetStringLibrary.Conv_IntToString` (`KismetArrayLibrary.Array_Length` (`self.AvailablePosition`))))
  (`self.RemoveAvailablePosition`))

(fn `GetRandomPosition`
  (returns (NewPosition :type "Vector Structure"))
  (locals (NewLocalVar :type "/Game/Procedural/Blueprint/BP_Cell Object Reference"))
  (return (`KismetArrayLibrary.Array_Random` (`self.AvailablePosition`))))

(fn `RemoveAvailablePosition`
  (bind _replacement (`self.Replacement`))
  (for _array_element (`self.AvailablePosition`)
    (for _array_element_2 (`self.ForbidenPosition`)
      (if (!= _array_element_2 _array_element :`ErrorTolerance` 1.0)
        (`KismetArrayLibrary.Array_AddUnique` _replacement _array_element)
        (else
          (`KismetArrayLibrary.Array_RemoveItem` _replacement _array_element)
          (break)))))
  (set `self.AvailablePosition` (`self.Replacement`))
  (`KismetArrayLibrary.Array_Clear` (`self.Replacement`)))

(fn `SetForbidenPosition`
  (for _array_element (`self.CellArray`)
    (`KismetArrayLibrary.Array_AddUnique` (`self.ForbidenPosition`) (`self.K2_GetActorLocation` _array_element)))
  (`self.AddAvailablePsoition`))

(fn `SpawnNewTile`
  (returns (ReturnValue :type "/Game/Procedural/Blueprint/BP_Cell Object Reference"))
  (bind _newposition (`self.GetRandomPosition`))
  (bind _returnvalue (`|SpawnActorFromClass` "/Game/Procedural/Blueprint/BP_Cell.BP_Cell_C" (`KismetMathLibrary.MakeTransform` _newposition) "Undefined" "MultiplyWithRoot" null null))
  (`KismetArrayLibrary.Array_AddUnique` (`self.CellArray`) _returnvalue)
  (`self.SetForbidenPosition`)
  (return null))

(fn `UserConstructionScript`)