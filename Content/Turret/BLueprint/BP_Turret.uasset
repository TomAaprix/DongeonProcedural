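; Turret actor that detects the first-person player within a view cone, turns toward them and applies damage.
; BeginPlay and every Tick trace from the muzzle, end the Niagara laser at the hit and compare the dot-product angle to the detection range.
; A trace hit on the player during detection re-sets a looping MakeDamage timer, never cleared here.
; Its health bar widget supplies Health and faces the player.
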(event `self.ReceiveBeginPlay`
  (`|ExecutionSequence`
    (:`then_0`
      (bind _aswbp_ui (cast `/Game/Turret/WBP_UI` (`WidgetComponent.GetUserWidgetObject` (`self.HealthBar`))))
      (set `self.Health` (`/Game/Turret/WBP_UI.Health` _aswbp_ui)))
    (:`then_1`
      (set `self.DirToPlayer` (- (`SceneComponent.K2_GetComponentLocation` (`Actor.RootComponent` (`GameplayStatics.GetPlayerCharacter` 0))) (`SceneComponent.K2_GetComponentLocation` (`self.ShootOrigin`))) :!label _label)
      (set `self.DirTurret` (`SceneComponent.GetForwardVector` (`self.ShootOrigin`)))
      (bind _outhit (`KismetSystemLibrary.LineTraceSingleForObjects` (`SceneComponent.K2_GetComponentLocation` (`self.ShootOrigin`)) (+ (* (`SceneComponent.GetForwardVector` (`self.ShootOrigin`)) (`self.MaxRange`)) (`SceneComponent.K2_GetComponentLocation` (`self.ShootOrigin`))) (`|MakeArray` "ObjectTypeQuery3" "ObjectTypeQuery4" "ObjectTypeQuery1" "ObjectTypeQuery2" :!type "EObjectTypeQuery Enum"))) ; Créer une ligne dans une direction depuis un point de départ
      (bind (_bblockinghit _binitialoverlap _time _distance _location _impactpoint _normal _impactnormal _physmat _hitactor) (`GameplayStatics.BreakHitResult` _outhit))
      ;[1 1 1] Affecte le lazer Niagara a la direction du vecteur
      (`FXSystemComponent.SetVectorParameter` (`self.NS_Lazer`) "EndBeam" _location)
      (if (<= (`KismetMathLibrary.DegAcos` (`KismetMathLibrary.Dot_VectorVector` (`KismetMathLibrary.Normal` (`self.DirToPlayer`)) (`KismetMathLibrary.Normal` (`self.DirTurret`)))) (`self.RangeDetection`))
        (`SceneComponent.K2_SetWorldRotation` (`self.Scene`) (`KismetMathLibrary.FindLookAtRotation` (`SceneComponent.K2_GetComponentLocation` (`self.Scene`)) (`SceneComponent.K2_GetComponentLocation` (`Actor.RootComponent` (`GameplayStatics.GetPlayerCharacter` 0)))) false false)
        (bind _asbp_first_person_character (cast `/Game/FirstPerson/Blueprints/BP_FirstPersonCharacter` _hitactor))
        (set `self.Player` _asbp_first_person_character)
        (`KismetSystemLibrary.K2_SetTimer` null "MakeDamage" 1.5 true)))))

(event `self.ReceiveTick`
  (params (DeltaSeconds :type "Float (single-precision)"))
  (bind _healthbar (`self.HealthBar`))
  (`SceneComponent.K2_SetWorldRotation` _healthbar (`KismetMathLibrary.FindLookAtRotation` (`SceneComponent.K2_GetComponentLocation` _healthbar) (`SceneComponent.K2_GetComponentLocation` (`Actor.RootComponent` (`GameplayStatics.GetPlayerCharacter` 0)))) false false)
  (goto _label))

(fn `MakeDamage`
  (bind _newhealth (`/Game/Turret/BPL_Health.TakeDammage` (`/Game/FirstPerson/Blueprints/BP_FirstPersonCharacter.Health` (`self.Player`)) (`self.Dammage`)))
  (set `/Game/FirstPerson/Blueprints/BP_FirstPersonCharacter.Health` _newhealth (`self.Player`)))

(fn `UserConstructionScript`)